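; BP_Marine is the player character, an armed marine with health, a kill counter and a HUD widget.
; Axis inputs move it along world X/Y, while mouse velocity beyond a dead zone smoothly turns the control yaw.
; Left click starts muzzle particles and sound until release, but fires only one damaging line trace from the muzzle socket per press.
; Incoming damage reduces health, and reaching zero sets Death, blocking movement, turning and firing.
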(event EventTick
  (params (DeltaSeconds :type Float%20%28single-precision%29))
  ;[1 1 1] movement
  (if (not (Variables|Default|GetDeath))
    (CallFunction|UpdatePlayerRotation)))

(event EventBeginPlay
  (bind _returnvalue (UserInterface|CreateWidget "/Game/UI/W_PlayerHUD.W_PlayerHUD_C" 0 self))
  (UserInterface|Viewport|AddtoViewport _returnvalue 0))

(event Game|Damage|EventAnyDamage
  (params (Damage :type Float%20%28single-precision%29) (DamageType :type Damage%20Type%20Object%20Reference) (InstigatedBy :type Controller%20Object%20Reference) (DamageCauser :type Actor%20Object%20Reference))
  ;[1 1 1] damage system
  (CallFunction|CheckPlayerDeath Damage))

(event Input|AxisEvents|InputAxisMoveForwardBack
  (params (AxisValue :type Float%20%28single-precision%29))
  ;[1 1 1] movement
  (if (not (Variables|Default|GetDeath))
    (Pawn|Input|AddMovementInput (Math|Vector|MakeVector AxisValue 0.0 0.0) 1.0 false)))

(event Input|AxisEvents|InputAxisMoveLeftRight
  (params (AxisValue :type Float%20%28single-precision%29))
  ;[1 1 1] movement
  (if (not (Variables|Default|GetDeath))
    (Pawn|Input|AddMovementInput (Math|Vector|MakeVector 0.0 AxisValue 0.0) 1.0 false)))

(event Input|MouseEvents|LeftMouseButton
  (params (Key :type Key%20Structure :default "None"))
  ;[1 1 1] shooting
  (:Pressed
    (if (not (Variables|Default|GetDeath))
      (CallFunction|ClicktoFire)
      (CallFunction|GenerateLinetrace)))
  (:Released
    (CallFunction|StopFire)
    (Audio|SpawnSound2D "/Game/Sounds/Weapon_AssaultRifle/Stereo/assault_riffle_end.assault_riffle_end" 1.0 1.0 0.0 0)))

(fn ConstructionScript)

(fn UpdatePlayerRotation
  (bind _returnvalue (CallFunction|GetMouseVelocity))
  (if (CallFunction|IsMouseDeadZone)
    (Pawn|SetControlRotation (Game|GetPlayerController 0) (Math|Interpolation|RInterpTo (Pawn|GetControlRotation :!class /Script/Engine.Pawn) (Math|Rotator|MakeRotator 0.0 0.0 (Class|KismetMathLibrary|DegAtan2 (.x _returnvalue) (.y _returnvalue))) (Utilities|Time|GetWorldDeltaSeconds) 1e+01))))

(fn GetMouseVelocity
  (bind _returnvalue (Game|GetPlayerController 0))
  (bind (_deltax _deltay) (Class|PlayerController|GetInputMouseDelta _returnvalue))
  (return (/ (Math|Vector2D|MakeVector2D _deltax _deltay) (Utilities|Time|GetWorldDeltaSeconds))))

(fn IsMouseDeadZone
  (return (> (Math|Vector2D|Vector2DLength (CallFunction|GetMouseVelocity)) (Variables|Default|Getmouse%20dead%20zone))))

(fn StopFire
  (Components|Activation|Deactivate (Variables|Default|GetP_AssaultRifle_MF))
  (if (not (Variables|Default|GetDeath))
    (Audio|Components|Audio|Stop (Variables|Default|Getweapon%20fire%20sound))))

(fn ClicktoFire
  (Components|Activation|Activate (Variables|Default|GetP_AssaultRifle_MF) false)
  (bind _returnvalue (Audio|SpawnSound2D "/Game/Sounds/Weapon_AssaultRifle/Stereo/assault_riffle.assault_riffle" 1.0 1.0 0.0 0))
  (Variables|Default|Setweapon%20fire%20sound _returnvalue))

(fn CheckPlayerDeath
  (params (Damage :type Float%20%28single-precision%29))
  (bind _output_get (Variables|Default|SetHealth (- (Variables|Default|GetHealth) Damage)))
  (if (== (Math|Float|Clamp(Float) _output_get 0.0 1e+02) 0.0)
    (bind _output_get_2 (Variables|Default|SetDeath true))
    (return _output_get_2)))

(fn GenerateLinetrace
  (bind _outhit (Collision|LineTraceByChannel (CallFunction|StartLocationLinetrace) (CallFunction|EndLocationLinetrace) "TraceTypeQuery1" false 0 "None"))
  (if (.bBlockingHit (Collision|BreakHitResult _outhit))
    (Game|Damage|ApplyDamage (.HitActor (Collision|BreakHitResult _outhit)) (Variables|Default|GetBase%20Damage) 0 0)))

(fn StartLocationLinetrace
  (return (Transformation|GetSocketLocation (Variables|Default|GetP_AssaultRifle_MF) "MuzzleFlashSocket")))

(fn EndLocationLinetrace
  (return (+ (* (Math|Vector|GetForwardVector (Transformation|GetSocketRotation (Variables|Default|GetP_AssaultRifle_MF) "MuzzleFlashSocket")) 2e+03) (CallFunction|StartLocationLinetrace))))

(fn IncreaseKills
  (Math|Integer|IncrementInt (Variables|Default|GetKills)
    (:%20%20
      (return))))

(fn GetKills
  (return (Variables|Default|GetKills)))